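; BP_Procedural_Mesh is a configurable modular-kit Blueprint that displays a chosen static mesh with a chosen material.
; Its construction script assigns the Mesh variable to the Cube component and applies MeshMaterial to the first material slot.
; It also reads the component's world scale and writes it back unchanged.
; Despite the name, it generates no geometry and has no active runtime logic.
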(fn ConstructionScript
  (bind _cube (Variables|Default|GetCube))
  (bind _cube_2 (Variables|Default|GetCube))
  (bind _returnvalue (Transformation|GetWorldScale _cube))
  (bind (_x _y _z) (Math|Vector|BreakVector _returnvalue))
  (Components|StaticMesh|SetStaticMesh _cube_2 (Variables|3D_params|GetMesh))
  (bind _output_get (Variables|3D_params|SetScale%20X _x))
  (bind _output_get_2 (Variables|3D_params|Set%20Scale%20Y _y))
  (bind _output_get_3 (Variables|3D_params|Set%20Scale%20Z _z))
  (Transformation|SetWorldScale3D _cube_2 (Math|Vector|MakeVector _output_get _output_get_2 _output_get_3))
  (Rendering|Material|SetMaterial _cube_2 0 (Variables|3D_params|GetMesh_Material)))

(fn ConstructionScript)