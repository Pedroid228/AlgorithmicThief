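; Modular kit constructor Blueprint that builds walls, corners, floors or rooms from one mesh in its Construction Script.
; It loops an X/Y/Z grid, and ConstructType picks the segment function that places instances along the relevant axes.
; InstancedParams derives placement from grid index, offsets and scaled mesh bounds, turning Y-only walls 90 degrees.
; MeshCreate adds a new instanced static mesh component for every cell, so instances are not batched grid-wide.
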(fn ConstructionScript
  (for _index (range 0 (- (Variables|Mesh_Operands|GetMesh_CountX) 1))
    (Variables|Indexes|SetX_Index _index)
    (for _index_2 (range 0 (- (Variables|Mesh_Operands|GetMesh_CountY) 1))
      (Variables|Indexes|SetY_Index _index_2)
      (for _index_3 (range 0 (- (Variables|Mesh_Operands|GetMesh_CountZ) 1))
        (Variables|Indexes|SetZ_Index _index_3)
        (CallFunction|MeshCreate)
        (switch Utilities|FlowControl|Switch|SwitchonENM_ConstructTypes (Variables|Mesh_Operands|GetConstruct_Type)
          (:NewEnumerator0
            (CallFunction|WallSegment))
          (:NewEnumerator1
            (CallFunction|CornerSegment))
          (:NewEnumerator2
            (CallFunction|FloorSegment))
          (:NewEnumerator3
            (CallFunction|RoomSegment)))))))

(fn InstancedParams
  (bind _mesh_scale (Variables|Mesh_Operands|GetMesh_Scale))
  (bind _mesh_rotator (Variables|Mesh_Operands|GetMesh_Rotator))
  (bind _mesh (Variables|Mesh_Operands|GetMesh))
  (bind _returnvalue (StaticMesh|GetBounds _mesh))
  (bind _returnvalue_2 (* _mesh_scale (.boxextent _returnvalue)))
  (bind (_x _y _z) (Math|Vector|BreakVector _returnvalue_2))
  (return (* (Math|Vector|MakeVector (* (* (Variables|Indexes|GetX_Index) (Variables|Mesh_Operands|GetX_Offset)) _x) (* (* (Variables|Indexes|GetY_Index) (Variables|Mesh_Operands|GetY_Offset)) (Math|Float|SelectFloat _x _y (>= _x _y))) (* (* (Variables|Indexes|GetZ_Index) (Variables|Mesh_Operands|GetZ_Offset)) _z)) 2.0) (Math|Rotator|SelectRotator (Math|Rotator|CombineRotators _mesh_rotator "0.000000,90.000000,0.000000") _mesh_rotator (Utilities|Select :Index (Variables|Mesh_Operands|GetConstruct_Type) :NewEnumerator0 (and (== (Variables|Mesh_Operands|GetX_Offset) 0) (!= 0 (Variables|Mesh_Operands|GetY_Offset))) :NewEnumerator1 false :NewEnumerator2 false :NewEnumerator3 false)) (Variables|Mesh_Operands|GetMesh_Scale)))

(fn MeshCreate
  (bind _returnvalue (AddComponent|AddInstancedStaticMeshComponent false))
  (bind _output_get (Variables|Default|SetInstance_Mesh _returnvalue))
  (Components|StaticMesh|SetStaticMesh _output_get (Variables|Mesh_Operands|GetMesh))
  (Rendering|Material|SetMaterial _output_get 0 (Variables|Mesh_Operands|GetMesh_Mat)))

(fn CornerSegment
  (bind (_mesh_location _mesh_rotation _mesh_scale) (CallFunction|InstancedParams))
  (bind (_x _y _z) (Math|Vector|BreakVector _mesh_location))
  (Utilities|FlowControl|Sequence
    (:then_0
      (Components|InstancedStaticMesh|AddInstance (Variables|Default|GetInstance_Mesh) (Math|Transform|MakeTransform (Math|Vector|MakeVector _x 0.0 _z) (Math|Rotator|CombineRotators _mesh_rotation (Math|Rotator|MakeRotator 0.0 0.0 (Math|Float|SelectFloat 0.0 1.8e+02 (> (Variables|Mesh_Operands|GetX_Offset) 0)))) _mesh_scale) false))
    (:then_1
      (Components|InstancedStaticMesh|AddInstance (Variables|Default|GetInstance_Mesh) (Math|Transform|MakeTransform (Math|Vector|MakeVector 0.0 _y _z) (Math|Rotator|CombineRotators _mesh_rotation (Math|Rotator|MakeRotator 0.0 0.0 (Math|Float|SelectFloat 9e+01 -9e+01 (> (Variables|Mesh_Operands|GetY_Offset) 0)))) _mesh_scale) false))))

(fn WallSegment
  (bind (_mesh_location _mesh_rotation _mesh_scale) (CallFunction|InstancedParams))
  (Components|InstancedStaticMesh|AddInstance (Variables|Default|GetInstance_Mesh) (Math|Transform|MakeTransform _mesh_location _mesh_rotation _mesh_scale) false))

(fn FloorSegment
  (bind (_mesh_location _mesh_rotation _mesh_scale) (CallFunction|InstancedParams))
  (Components|InstancedStaticMesh|AddInstance (Variables|Default|GetInstance_Mesh) (Math|Transform|MakeTransform (Math|Vector|MakeVector (.x _mesh_location) (.y _mesh_location) 0.0) _mesh_rotation _mesh_scale) false))

(fn RoomSegment
  (bind (_mesh_location _mesh_rotation _mesh_scale) (CallFunction|InstancedParams))
  (bind (_mesh_location_2 _mesh_rotation_2 _mesh_scale_2) (CallFunction|InstancedParams))
  (bind _instance_mesh (Variables|Default|GetInstance_Mesh))
  (bind _instance_mesh_2 (Variables|Default|GetInstance_Mesh))
  (bind (_x _y) (Math|Vector|BreakVector _mesh_location))
  (bind (_x_2 _y_2 _z) (Math|Vector|BreakVector _mesh_location_2))
  (Utilities|FlowControl|Sequence
    (:then_0
      (Components|InstancedStaticMesh|AddInstance _instance_mesh (Math|Transform|MakeTransform (Math|Vector|MakeVector _x_2 0.0 _z) _mesh_rotation_2 _mesh_scale_2) false))
    (:then_1
      (Components|InstancedStaticMesh|AddInstance _instance_mesh (Math|Transform|MakeTransform (Math|Vector|MakeVector 0.0 _y_2 _z) (Math|Rotator|CombineRotators _mesh_rotation_2 "0.000000,-90.000000,0.000000") _mesh_scale_2) false))
    (:then_2
      (Components|InstancedStaticMesh|AddInstance _instance_mesh_2 (Math|Transform|MakeTransform (Math|Vector|MakeVector _y 0.0 0.0) _mesh_rotation _mesh_scale) false))
    (:then_3
      (Components|InstancedStaticMesh|AddInstance _instance_mesh_2 (Math|Transform|MakeTransform (Math|Vector|MakeVector 0.0 _x 0.0) _mesh_rotation _mesh_scale) false))))

(fn AxisRotators
  (switch Utilities|FlowControl|Switch|SwitchonENM_ConstructTypes (Variables|Mesh_Operands|GetConstruct_Type)
    (:NewEnumerator0
      (return "0, 0, 0"))
    (:NewEnumerator1
      (return "0, 0, 0"))))