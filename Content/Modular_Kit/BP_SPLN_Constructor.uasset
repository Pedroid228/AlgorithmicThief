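; Modular kit Blueprint that tiles a chosen mesh along a spline as deformed spline mesh segments with collision.
; The construction script derives segment length from the mesh's X bounds, then adds segments along the spline with a set material and forward axis.
; Tangents are clamped to segment length, and Limitter scales only each segment's start distance.
; SPLLOCATION returns the world position of the spline point indexed by SPLINEPNT.
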(fn ConstructionScript
  (bind _spl_mesh (Variables|Mesh_Params|GetSPL_Mesh))
  (bind _spline (Variables|Default|GetSpline))
  (bind _spline_2 (Variables|Default|GetSpline))
  (bind _returnvalue (StaticMesh|GetBoundingBox _spl_mesh))
  (bind _output_get (Variables|Default|SetX_Length (.x (+ (Math|Vector|VectorGetAbs (.min _returnvalue)) (Math|Vector|VectorGetAbs (.max _returnvalue))))))
  (for _index (range 0 (Math|Float|Truncate (/ (Spline|GetSplineLength (Variables|Default|GetSpline)) _output_get)))
    (bind _returnvalue_2 (AddComponent|AddSplineMeshComponent false))
    (Components|StaticMesh|SetStaticMesh _returnvalue_2 (Variables|Mesh_Params|GetSPL_Mesh))
    (Rendering|Material|SetMaterial _returnvalue_2 0 (Variables|Mesh_Params|GetM_Mat))
    (SplineMesh|SetForwardAxis _returnvalue_2 (Variables|Mesh_Params|GetForward%20Axis) true)
    (Collision|SetCollisionEnabled _returnvalue_2 "QueryAndPhysics")
    (SplineMesh|SetStartandEnd _returnvalue_2 (Spline|GetLocationatDistanceAlongSpline _spline_2 (* _index (* (Variables|Default|GetX_Length) (Variables|Default|GetLimitter))) "Local") (Math|Vector|ClampVectorSize (Spline|GetTangentatDistanceAlongSpline _spline_2 (* _index (* (Variables|Default|GetX_Length) (Variables|Default|GetLimitter))) "Local") 0.0 (Variables|Default|GetX_Length)) (Spline|GetLocationatDistanceAlongSpline _spline (* (+ _index 1) (Variables|Default|GetX_Length)) "Local") (Math|Vector|ClampVectorSize (Spline|GetTangentatDistanceAlongSpline _spline (* (+ _index 1) (Variables|Default|GetX_Length)) "Local") 0.0 (Variables|Default|GetX_Length)) true :!class /Script/Engine.SplineMeshComponent)))

(fn SPLLOCATION
  (return (Spline|GetLocationatSplinePoint (Variables|Default|GetSpline) (Variables|Default|GetSPLINE_PNT) "World")))