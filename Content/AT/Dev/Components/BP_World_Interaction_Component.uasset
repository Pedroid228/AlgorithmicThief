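; A world interaction component that detects which interactable actor its owner is pointing at and sends hover messages to it.
; An externally called Trace event runs a debug-drawn Visibility line trace from a given start, direction and length, ignoring the owner.
; A new hit implementing BP_World_Interaction_Interface becomes HoveredActor and receives OnHovered with the owner.
; Unhover fires only when the trace hits nothing, not when it moves to another actor.
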(event Custom|Trace
  (params (Start_In :type Vector) (Direction_In :type Vector) (Length_In :type Float%20%28double-precision%29))
  (bind (_outhit _returnvalue) (Collision|LineTraceByChannel Start_In (+ Start_In (* (Math|Vector|Normalize Direction_In) Length_In)) "TraceTypeQuery1" false (Utilities|Array|MakeArray (Components|GetOwner)) "ForOneFrame"))
  (if _returnvalue
    (if (Utilities|DoesObjectImplementInterface (.HitActor (Collision|BreakHitResult _outhit)) "/Game/AT/Dev/Interfaces/BP_World_Interaction_Interface.BP_World_Interaction_Interface_C")
      (if (!= (Variables|Default|GetHovered_Actor) (.HitActor (Collision|BreakHitResult _outhit)))
        (bind _output_get (Variables|Default|SetHovered_Actor (.HitActor (Collision|BreakHitResult _outhit))))
        (Class|BPWorldInteractionInterface|OnHovered(Message) _output_get (Components|GetOwner))))
    (else
      (Utilities|IsValid (Variables|Default|GetHovered_Actor)
        (:Is%20Valid
          (Class|BPWorldInteractionInterface|OnUnhovered(Message) (Variables|Default|GetHovered_Actor))
          (Variables|Default|SetHovered_Actor 0))))))

(event EventBeginPlay)

(event EventTick
  (params (DeltaSeconds :type Float%20%28single-precision%29)))