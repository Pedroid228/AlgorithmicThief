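; Visor component that reveals the most valuable diamonds in the level by highlighting them for a given time.
; GreedyScan gathers all BP_Diamond actors and makes a single pass over those not in a bag, tracking the highest price and keeping every diamond tied at it.
; Each diamond in that best set then activates its own timed highlight.
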(event EventBeginPlay)

(event EventTick
  (params (DeltaSeconds :type Float%20%28single-precision%29)))

(fn GreedyScan
  (params (Highlight_Time :type Float%20%28double-precision%29))
  (Utilities|Array|Clear (Variables|Default|GetBest_Diamonds))
  (bind _outactors (Actor|GetAllActorsOfClass "/Game/AT/Dev/Diamond/BP_Diamond.BP_Diamond_C"))
  (Variables|Default|SetDiamonds _outactors)
  (for _array_element (Variables|Default|GetDiamonds)
    (bind _output_get (Variables|Default|SetCurr_Diamond _array_element))
    (if (not (Variables|/Game/AT/Dev/Diamond/BP_Diamond.BP_Diamond_C|GetIs_In_Bag _output_get))
      (if (== (Utilities|Array|Length (Variables|Default|GetBest_Diamonds)) 0)
        ;[1 1 1] First diamond as best OR new best
        (Utilities|Array|Clear (Variables|Default|GetBest_Diamonds) :!label _label)
        (Utilities|Array|Add (Variables|Default|GetBest_Diamonds) (Variables|Default|GetCurr_Diamond))
        (Variables|Default|SetBest_Diamond_Price (.Price (Utilities|Struct|BreakSDiamond_Data (Variables|/Game/AT/Dev/Diamond/BP_Diamond.BP_Diamond_C|GetDiamond_Data (Variables|Default|GetCurr_Diamond)))))
        (elif (> (.Price (Utilities|Struct|BreakSDiamond_Data (Variables|/Game/AT/Dev/Diamond/BP_Diamond.BP_Diamond_C|GetDiamond_Data (Variables|Default|GetCurr_Diamond)))) (Variables|Default|GetBest_Diamond_Price))
          (goto _label)
          (else
            ;[1 1 1] Add curr diamond to best diamonds
            (if (== (.Price (Utilities|Struct|BreakSDiamond_Data (Variables|/Game/AT/Dev/Diamond/BP_Diamond.BP_Diamond_C|GetDiamond_Data (Variables|Default|GetCurr_Diamond)))) (Variables|Default|GetBest_Diamond_Price))
              (Utilities|Array|Add (Variables|Default|GetBest_Diamonds) (Variables|Default|GetCurr_Diamond))))))))
  (for _array_element_2 (Variables|Default|GetBest_Diamonds)
    (Default|ActivateHighlightonTime _array_element_2 Highlight_Time)))