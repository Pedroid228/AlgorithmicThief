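; BP_Qick_Sort_Manager runs an interactive quicksort puzzle where grabbable diamonds on platforms are partitioned by price.
; The root spawns the platforms and diamonds, and Start_Sort picks a random pivot and shifts platforms to match each partition's size.
; Once both sides hold the correct diamonds, it notifies GM_Qick_Sort, separates the platforms and recursively spawns two child managers.
; When every platform has been a pivot, the root realigns them and enables bag collection.
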(event Custom|Check_Pivot_Platforms_Cnt
  (if (Variables|Default|GetIs_Root_Manager)
    (bind _result (Math|Integer|IncrementInt (Variables|Default|GetPivot_Platforms_Cnt))
      (:%20%20
        (if (>= _result (Utilities|Array|Length (Variables|Default|GetPlatforms)))
          (bind _asat_game_instance (Utilities|Casting|CastToAT_Game_Instance (Game|GetGameInstance)))
          (Default|PlayHelperSoundbyActionSort _asat_game_instance "NewEnumerator10")
          (bind _outactors (Actor|GetAllActorsOfClass "/Game/AT/Dev/Bag/BP_Bag.BP_Bag_C"))
          (Variables|/Game/AT/Dev/Bag/BP_Bag.BP_Bag_C|SetCan_Add_Diamond_In_Lab (Utilities|Array|Get(acopy) _outactors) true)
          (for _array_element (Variables|Default|GetPlatforms)
            (Default|MoveinDirection _array_element "NewEnumerator0" (* (Math|Float|Absolute(Float) (.y (- (Transformation|GetActorLocation _array_element) (Transformation|GetActorLocation)))) -1.0))
            (Variables|/Game/AT/Dev/Diamond/BP_Diamond.BP_Diamond_C|SetCan_Be_Grabbed_Flag (Variables|/Game/AT/Dev/Quick_Sort/BP_Diamond_Platform.BP_Diamond_Platform_C|GetContained_Diamond _array_element) true)))))))

(event Custom|Start_Sort
  (CallFunction|QuickSort (Variables|Default|GetPlatforms)))

(event EventBeginPlay
  (if (Variables|Default|GetIs_Root_Manager)
    (for (_array_element _array_index) (Variables|Default|GetShufled_Bag_Diamonds)
      (Variables|Default|SetCurr_Diamond_Data _array_element)
      (Variables|Default|SetCurr_Platform_Index _array_index)
      (bind _returnvalue (Game|SpawnActorfromClass "/Game/AT/Dev/Quick_Sort/BP_Diamond_Platform.BP_Diamond_Platform_C" (Math|Transform|MakeTransform (+ (Transformation|GetActorLocation) (* (Transformation|GetActorForwardVector) (Variables|Default|GetPlatforms_Distance) (Variables|Default|GetCurr_Platform_Index)))) "Undefined" "MultiplyWithRoot" 0 0))
      (bind _output_get (Variables|Default|SetCurr_Platform _returnvalue))
      (EventDispatchers|BindEventtoOnSetasPivot _output_get (delegate Custom|Check_Pivot_Platforms_Cnt))
      (Utilities|Array|Add (Variables|Default|GetPlatforms) (Variables|Default|GetCurr_Platform))
      (bind _returnvalue_2 (Game|SpawnActorfromClass "/Game/AT/Dev/Diamond/BP_Diamond.BP_Diamond_C" (Math|Transform|MakeTransform "0, 0, 0") "Undefined" "MultiplyWithRoot" 0 0))
      (Variables|/Game/AT/Dev/Diamond/BP_Diamond.BP_Diamond_C|SetDiamond_Data _returnvalue_2 (Variables|Default|GetCurr_Diamond_Data))
      (Default|OnDeadZoneBeginOverlap (Variables|Default|GetCurr_Platform) 0 _returnvalue_2 0 0 false)
      (Rendering|Components|TextRender|SetText (Variables|/Game/AT/Dev/Diamond/BP_Diamond.BP_Diamond_C|GetPrice_Text _returnvalue_2) (Utilities|Text|ToText(Float) (.price (Variables|Default|GetCurr_Diamond_Data)) "HalfToEven"))
      (Variables|/Game/AT/Dev/Diamond/BP_Diamond.BP_Diamond_C|SetCan_Be_Grabbed_Flag _returnvalue_2 false))))

(event Collision|EventActorBeginOverlap
  (params (OtherActor :type Actor%20Object%20Reference)))

(event EventTick
  (params (DeltaSeconds :type Float%20%28single-precision%29)))

(fn ConstructionScript)

(fn QuickSort
  (params (Sorting_Platforms :type Array%20of%20BP%20Diamond%20Platform%20Object%20References))
  (bind _after_pivot_platforms_cnt (LocalVariables|GetAfter_Pivot_Platforms_Cnt))
  (bind _target_greater_string (Variables|Default|GetTarget_Greater_String))
  (bind _returnvalue (Utilities|Set|Length _target_greater_string))
  (bind _returnvalue_2 (- _returnvalue _after_pivot_platforms_cnt))
  (bind _returnvalue_3 (Math|Integer|Absolute(Integer) _returnvalue_2))
  (LocalVariables|SetSorting_Platforms_Local Sorting_Platforms)
  (Utilities|Array|Clear (Variables|Default|GetFlying_Platforms))
  (Utilities|Set|Clear (Variables|Default|GetTarget_Less_String))
  (Utilities|Set|Clear (Variables|Default|GetTarget_Greater_String))
  (bind _output_get (LocalVariables|SetSorting_Platforms_Len (Utilities|Array|Length (LocalVariables|GetSorting_Platforms_Local))))
  (if (!= _output_get 0)
    (if (!= (LocalVariables|GetSorting_Platforms_Len) 1)
      (Variables|Default|SetPivot_Index (Math|Random|RandomIntegerinRange 1 (- (LocalVariables|GetSorting_Platforms_Len) 2)))
      (else
        (Variables|Default|SetPivot_Index 0)))
    (bind _output_get_2 (LocalVariables|SetPivot_Platform (Utilities|Array|Get(acopy) (LocalVariables|GetSorting_Platforms_Local) (Variables|Default|GetPivot_Index))))
    (Default|SetasPivot _output_get_2)
    (if (not (< (LocalVariables|GetSorting_Platforms_Len) 2))
      (for (_array_element _array_index) (LocalVariables|GetSorting_Platforms_Local)
        (bind _output_get_3 (LocalVariables|SetCurr_Platform_Index_Local _array_index))
        (if (!= _output_get_3 (Variables|Default|GetPivot_Index))
          (bind _output_get_4 (LocalVariables|SetCurr_Sorting_Platform _array_element))
          (EventDispatchers|UnbindallEventsfromOnStopMoving _output_get_4)
          (EventDispatchers|UnbindallEventsfromOnDiamondAttachedDispatcher _output_get_4)
          (EventDispatchers|BindEventtoOnDiamondAttachedDispatcher _output_get_4 (EventDispatchers|CreateEvent :!event CheckString))
          ;[1 1 1] Separate platforms on two groups: BEFORE pivot and AFTER pivot
          (if (< (LocalVariables|GetCurr_Platform_Index_Local) (Variables|Default|GetPivot_Index))
            (Variables|/Game/AT/Dev/Quick_Sort/BP_Diamond_Platform.BP_Diamond_Platform_C|SetIs_After_Pivot (LocalVariables|GetCurr_Sorting_Platform) true)
            (Math|Integer|IncrementInt (LocalVariables|GetAfter_Pivot_Platforms_Cnt)
              (:%20%20
                _))
            (else
              (Variables|/Game/AT/Dev/Quick_Sort/BP_Diamond_Platform.BP_Diamond_Platform_C|SetIs_After_Pivot (LocalVariables|GetCurr_Sorting_Platform) false)))
          ;[1 1 1] Sort diamonds to LESS and GREATER than pivots sets
          (Utilities|IsValid (Variables|/Game/AT/Dev/Quick_Sort/BP_Diamond_Platform.BP_Diamond_Platform_C|GetContained_Diamond (LocalVariables|GetCurr_Sorting_Platform))
            (:Is%20Valid
              (LocalVariables|SetCurr_Platform_Diamond (Variables|/Game/AT/Dev/Quick_Sort/BP_Diamond_Platform.BP_Diamond_Platform_C|GetContained_Diamond (LocalVariables|GetCurr_Sorting_Platform)))
              (if (<= (.Price (Utilities|Struct|BreakSDiamond_Data (Variables|/Game/AT/Dev/Diamond/BP_Diamond.BP_Diamond_C|GetDiamond_Data (LocalVariables|GetCurr_Platform_Diamond)))) (.Price (Utilities|Struct|BreakSDiamond_Data (Variables|/Game/AT/Dev/Diamond/BP_Diamond.BP_Diamond_C|GetDiamond_Data (Variables|/Game/AT/Dev/Quick_Sort/BP_Diamond_Platform.BP_Diamond_Platform_C|GetContained_Diamond (LocalVariables|GetPivot_Platform))))))
                (Utilities|Set|Add (Variables|Default|GetTarget_Less_String) (LocalVariables|GetCurr_Platform_Diamond))
                (else
                  (Utilities|Set|Add (Variables|Default|GetTarget_Greater_String) (LocalVariables|GetCurr_Platform_Diamond)))))
            (:Is%20Not%20Valid
              (Development|PrintString "ERROR Platform dont have diamond" true true "(R=1.000000,G=0.017512,B=0.000000,A=1.000000)")))))
      ;[1 1 1] Move platforms relative of pivot
      (if (!= _returnvalue_2 0)
        (Variables|Default|SetIs_Moving_Platforms_After_Pivot (> _returnvalue_2 0))
        (Variables|Default|SetMoving_To_First_Platforms_Cnt _returnvalue_3)
        (CallFunction|SetCanGrabDiamonds false)
        (for _index (range 0 (- _returnvalue_3 1))
          (bind _output_get_5 (LocalVariables|SetCurr_Platform_Index_Local _index))
          (Utilities|Array|Add (Variables|Default|GetFlying_Platforms) (Utilities|Array|Get(acopy) (LocalVariables|GetSorting_Platforms_Local) (Math|Integer|SelectInt (- (- (Utilities|Array|Length (LocalVariables|GetSorting_Platforms_Local)) 1) (LocalVariables|GetCurr_Platform_Index_Local)) _output_get_5 (Variables|Default|GetIs_Moving_Platforms_After_Pivot))))
          (Variables|/Game/AT/Dev/Quick_Sort/BP_Diamond_Platform.BP_Diamond_Platform_C|SetIs_After_Pivot (Utilities|Array|Get(acopy) (LocalVariables|GetSorting_Platforms_Local) (Math|Integer|SelectInt (- (- (Utilities|Array|Length (LocalVariables|GetSorting_Platforms_Local)) 1) (LocalVariables|GetCurr_Platform_Index_Local)) _output_get_5 (Variables|Default|GetIs_Moving_Platforms_After_Pivot))) (not (Variables|/Game/AT/Dev/Quick_Sort/BP_Diamond_Platform.BP_Diamond_Platform_C|GetIs_After_Pivot (Utilities|Array|Get(acopy) (LocalVariables|GetSorting_Platforms_Local) (Math|Integer|SelectInt (- (- (Utilities|Array|Length (LocalVariables|GetSorting_Platforms_Local)) 1) (LocalVariables|GetCurr_Platform_Index_Local)) _output_get_5 (Variables|Default|GetIs_Moving_Platforms_After_Pivot))))))
          (Default|MoveinFirstPos (Utilities|Array|Get(acopy) (LocalVariables|GetSorting_Platforms_Local) (Math|Integer|SelectInt (- (- (Utilities|Array|Length (LocalVariables|GetSorting_Platforms_Local)) 1) (LocalVariables|GetCurr_Platform_Index_Local)) _output_get_5 (Variables|Default|GetIs_Moving_Platforms_After_Pivot))) (* (+ (* (+ (LocalVariables|GetCurr_Platform_Index_Local) 1) (Variables|Default|GetPlatforms_Distance)) (Math|Vector|Distance(Vector) (Transformation|GetActorLocation (Utilities|Array|Get(acopy) (LocalVariables|GetSorting_Platforms_Local) (Math|Integer|SelectInt (- (- (Utilities|Array|Length (LocalVariables|GetSorting_Platforms_Local)) 1) (LocalVariables|GetCurr_Platform_Index_Local)) _output_get_5 (Variables|Default|GetIs_Moving_Platforms_After_Pivot)))) (Transformation|GetActorLocation (Utilities|Array|Get(acopy) (LocalVariables|GetSorting_Platforms_Local) (Math|Integer|SelectInt 0 (- (Utilities|Array|Length (LocalVariables|GetSorting_Platforms_Local)) 1) (Variables|Default|GetIs_Moving_Platforms_After_Pivot)))))) (Math|Integer|SelectInt -1 1 (Variables|Default|GetIs_Moving_Platforms_After_Pivot))) (Variables|Default|GetForward_Move_Distance) (Variables|Default|GetUp_Move_Distance))
          (EventDispatchers|BindEventtoOnStopRebuild (Utilities|Array|Get(acopy) (LocalVariables|GetSorting_Platforms_Local) (Math|Integer|SelectInt (- (- (Utilities|Array|Length (LocalVariables|GetSorting_Platforms_Local)) 1) (LocalVariables|GetCurr_Platform_Index_Local)) _output_get_5 (Variables|Default|GetIs_Moving_Platforms_After_Pivot))) (EventDispatchers|CreateEvent :!event StopRebuildHandler)))
        (else
          (CallFunction|SetCanGrabDiamonds true)
          (CallFunction|CheckString))))))

(fn CheckString
  (for _index (range 0 (- (Utilities|Array|Length (Variables|Default|GetPlatforms)) 1))
    (if (!= _index (Variables|Default|GetPivot_Index))
      (LocalVariables|SetCurr_Platform_Local (Utilities|Array|Get(acopy) (Variables|Default|GetPlatforms) _index))
      (if (Variables|/Game/AT/Dev/Quick_Sort/BP_Diamond_Platform.BP_Diamond_Platform_C|GetIs_After_Pivot (LocalVariables|GetCurr_Platform_Local))
        (Utilities|IsValid (Variables|/Game/AT/Dev/Quick_Sort/BP_Diamond_Platform.BP_Diamond_Platform_C|GetContained_Diamond (LocalVariables|GetCurr_Platform_Local))
          (:Is%20Valid
            (Utilities|Set|Add (LocalVariables|GetCurr_Greater_String) (Variables|/Game/AT/Dev/Quick_Sort/BP_Diamond_Platform.BP_Diamond_Platform_C|GetContained_Diamond (LocalVariables|GetCurr_Platform_Local)))))
        (else
          (Utilities|IsValid (Variables|/Game/AT/Dev/Quick_Sort/BP_Diamond_Platform.BP_Diamond_Platform_C|GetContained_Diamond (LocalVariables|GetCurr_Platform_Local))
            (:Is%20Valid
              (Utilities|Set|Add (LocalVariables|GetCurr_Less_String) (Variables|/Game/AT/Dev/Quick_Sort/BP_Diamond_Platform.BP_Diamond_Platform_C|GetContained_Diamond (LocalVariables|GetCurr_Platform_Local)))))))))
  (bind _result (Utilities|Set|Difference (Variables|Default|GetTarget_Less_String) (LocalVariables|GetCurr_Less_String)))
  (bind _result_2 (Utilities|Set|Difference (LocalVariables|GetCurr_Less_String) (Variables|Default|GetTarget_Less_String)))
  (bind _result_3 (Utilities|Set|Difference (Variables|Default|GetTarget_Greater_String) (LocalVariables|GetCurr_Greater_String)))
  (bind _result_4 (Utilities|Set|Difference (LocalVariables|GetCurr_Greater_String) (Variables|Default|GetTarget_Greater_String)))
  (if (and (and (== (Utilities|Set|Length _result_4) 0) (== (Utilities|Set|Length _result_3) 0)) (and (== (Utilities|Set|Length _result_2) 0) (== (Utilities|Set|Length _result) 0)))
    (CallFunction|SetCanGrabDiamonds false)
    (bind _asgm_qick_sort (Utilities|Casting|CastToGM_Qick_Sort (Game|GetGameMode)))
    (Default|OnStringComplete _asgm_qick_sort)
    (for (_array_element _array_index) (Variables|Default|GetPlatforms)
      (if (!= _array_index (Variables|Default|GetPivot_Index))
        (EventDispatchers|UnbindallEventsfromOnStopMoving _array_element)
        (EventDispatchers|BindEventtoOnStopMoving _array_element (EventDispatchers|CreateEvent :!event CreateChildren))
        (Default|MoveinDirection _array_element "NewEnumerator0" (Variables|Default|GetForward_Move_Distance))))))

(fn StopRebuildHandler
  (params (Platform :type BP%20Diamond%20Platform%20Object%20Reference))
  (Math|Integer|IncrementInt (Variables|Default|GetMoved_Platforms)
    (:%20%20
      (if (>= (Variables|Default|GetMoved_Platforms) (Variables|Default|GetMoving_To_First_Platforms_Cnt))
        (for _array_element (Variables|Default|GetPlatforms)
          (LocalVariables|SetCurr_Platform _array_element)
          (Default|MoveinDirection (LocalVariables|GetCurr_Platform) "NewEnumerator1" (* (Variables|Default|GetPlatforms_Distance) (Variables|Default|GetMoving_To_First_Platforms_Cnt) (Math|Integer|SelectInt 1 -1 (Variables|Default|GetIs_Moving_Platforms_After_Pivot))))
          (EventDispatchers|UnbindallEventsfromOnStopRebuild (LocalVariables|GetCurr_Platform))
          (EventDispatchers|BindEventtoOnStopMoving (LocalVariables|GetCurr_Platform) (EventDispatchers|CreateEvent :!event OnStopAligment)))))))

(fn Setup
  (params (Platforms :type Array%20of%20BP%20Diamond%20Platform%20Object%20References) (Platforms_Distance :type Float%20%28double-precision%29) (Forward_Move_Distance :type Float%20%28double-precision%29))
  (Variables|Default|SetPlatforms Platforms)
  (Variables|Default|SetPlatforms_Distance Platforms_Distance)
  (Variables|Default|SetForward_Move_Distance Forward_Move_Distance)
  (CallFunction|QuickSort (Variables|Default|GetPlatforms)))

(fn CreateChildren
  (for (_array_element _array_index) (Variables|Default|GetPlatforms)
    (LocalVariables|SetCurr_Platform _array_element)
    (if (!= _array_index (Variables|Default|GetPivot_Index))
      (EventDispatchers|UnbindallEventsfromOnStopMoving (LocalVariables|GetCurr_Platform))
      (EventDispatchers|UnbindallEventsfromOnDiamondAttachedDispatcher (LocalVariables|GetCurr_Platform))
      (if (Variables|/Game/AT/Dev/Quick_Sort/BP_Diamond_Platform.BP_Diamond_Platform_C|GetIs_After_Pivot (LocalVariables|GetCurr_Platform))
        (Utilities|Map|Add (LocalVariables|GetAfter_Pivot_Hash_Map) (Math|Vector|Distance(Vector) (Transformation|GetActorLocation (LocalVariables|GetCurr_Platform)) (Transformation|GetActorLocation (Utilities|Array|Get(acopy) (Variables|Default|GetPlatforms) (Variables|Default|GetPivot_Index)))) (LocalVariables|GetCurr_Platform))
        (Utilities|Array|Add (LocalVariables|GetAfter_Pivot_Distances) (Math|Vector|Distance(Vector) (Transformation|GetActorLocation (LocalVariables|GetCurr_Platform)) (Transformation|GetActorLocation (Utilities|Array|Get(acopy) (Variables|Default|GetPlatforms) (Variables|Default|GetPivot_Index)))))
        (else
          (Utilities|Map|Add (LocalVariables|GetBefore_Pivot_Hash_Map) (Math|Vector|Distance(Vector) (Transformation|GetActorLocation (LocalVariables|GetCurr_Platform)) (Transformation|GetActorLocation (Utilities|Array|Get(acopy) (Variables|Default|GetPlatforms) (Variables|Default|GetPivot_Index)))) (LocalVariables|GetCurr_Platform))
          (Utilities|Array|Add (LocalVariables|GetBefore_Pivot_Distances) (Math|Vector|Distance(Vector) (Transformation|GetActorLocation (LocalVariables|GetCurr_Platform)) (Transformation|GetActorLocation (Utilities|Array|Get(acopy) (Variables|Default|GetPlatforms) (Variables|Default|GetPivot_Index)))))))))
  (Class|KismetArrayLibrary|SortFloatArray (LocalVariables|GetAfter_Pivot_Distances) false "Descending")
  (Class|KismetArrayLibrary|SortFloatArray (LocalVariables|GetBefore_Pivot_Distances))
  (Utilities|FlowControl|Sequence
    (:then_0
      (for _array_element_2 (LocalVariables|GetAfter_Pivot_Distances)
        (if (.ReturnValue (Utilities|Map|Find (LocalVariables|GetAfter_Pivot_Hash_Map) _array_element_2))
          (Utilities|Array|Add (LocalVariables|GetAfter_Pivot_Platforms) (.Value (Utilities|Map|Find (LocalVariables|GetAfter_Pivot_Hash_Map) _array_element_2))))))
    (:then_1
      (for _array_element_3 (LocalVariables|GetBefore_Pivot_Distances)
        (if (.ReturnValue (Utilities|Map|Find (LocalVariables|GetBefore_Pivot_Hash_Map) _array_element_3))
          (Utilities|Array|Add (LocalVariables|GetBefore_Pivot_Platforms) (.Value (Utilities|Map|Find (LocalVariables|GetBefore_Pivot_Hash_Map) _array_element_3))))))
    (:then_2
      (bind _returnvalue (Game|SpawnActorfromClass "BP_Qick_Sort_Manager_C" (Math|Transform|MakeTransform "0, 0, 0") "Undefined" "MultiplyWithRoot" 0 false 0))
      (CallFunction|Setup _returnvalue (LocalVariables|GetBefore_Pivot_Platforms) (Variables|Default|GetPlatforms_Distance) (Variables|Default|GetForward_Move_Distance))
      (bind _returnvalue_2 (Game|SpawnActorfromClass "BP_Qick_Sort_Manager_C" (Math|Transform|MakeTransform "0, 0, 0") "Undefined" "MultiplyWithRoot" 0 false 0))
      (CallFunction|Setup _returnvalue_2 (LocalVariables|GetAfter_Pivot_Platforms) (Variables|Default|GetPlatforms_Distance) (Variables|Default|GetForward_Move_Distance)))))

(fn OnStopAligment
  (CallFunction|SetCanGrabDiamonds true)
  (for _array_element (Variables|Default|GetPlatforms)
    (EventDispatchers|UnbindallEventsfromOnStopMoving _array_element))
  (for _array_element_2 (Variables|Default|GetFlying_Platforms)
    (EventDispatchers|BindEventtoOnStopMoving _array_element_2 (EventDispatchers|CreateEvent :!event CheckString))
    (Default|MoveinDirection _array_element_2 "NewEnumerator4" (* (Variables|Default|GetUp_Move_Distance) -1.0))))

(fn SetCanGrabDiamonds
  (params (Can_Grab :type Boolean))
  (for (_array_element _array_index) (Variables|Default|GetPlatforms)
    (if (!= _array_index (Variables|Default|GetPivot_Index))
      (Utilities|IsValid (Variables|/Game/AT/Dev/Quick_Sort/BP_Diamond_Platform.BP_Diamond_Platform_C|GetContained_Diamond _array_element)
        (:Is%20Valid
          (Variables|/Game/AT/Dev/Diamond/BP_Diamond.BP_Diamond_C|SetCan_Be_Grabbed_Flag (Variables|/Game/AT/Dev/Quick_Sort/BP_Diamond_Platform.BP_Diamond_Platform_C|GetContained_Diamond _array_element) Can_Grab))))))

(fn EndSeparation
  (for _array_element (Variables|Default|GetPlatforms)
    (EventDispatchers|UnbindallEventsfromOnStopMoving _array_element))
  (CallFunction|CreateChildren))