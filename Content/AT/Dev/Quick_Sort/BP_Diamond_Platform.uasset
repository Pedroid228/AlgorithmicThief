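; Diamond platform for a Quick Sort puzzle, holding one diamond that can be marked as pivot and repositioning itself during rebuilds.
; While empty, Tick snaps any ungrabbed diamond in the DeadZone to its socket.
; A capsule overlap with the thief toggles whether that diamond can be grabbed.
; Rebuilds step through an enum state machine of up, back, side and forward VInterpTo moves, with dispatchers announcing changes.
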(event Custom|Move_In_First_Pos
  (params (Side_Move_Distance :type Float%20%28double-precision%29) (Back_Move_Distance :type Float%20%28double-precision%29) (Up_Move_Distance :type Float%20%28double-precision%29))
  (Variables|Default|SetSide_Move_Distance_Local Side_Move_Distance)
  (Variables|Default|SetBack_Move_Distance_Local Back_Move_Distance)
  (Variables|Default|SetUp_Move_Distance_Local Up_Move_Distance)
  (CallFunction|SetNewStringRebuildState "NewEnumerator4"))

(event Custom|On_Attach_Diamond
  (params (Instigator :type BP%20Diamond%20Object%20Reference))
  (bind _output_get (Variables|Default|SetContained_Diamond Instigator))
  (CallFunction|AttachDiamond _output_get)
  (Variables|Default|SetHas_Diamond true)
  (Default|CallOnDiamondAttachedDispatcher)
  (EventDispatchers|BindEventtoOnGrabbedDispatcher (Variables|Default|GetContained_Diamond) (delegate Custom|On_Attached_Diamond_Grabbed))
  (if (Variables|Default|GetIs_Player_In_Capsule)
    (Variables|/Game/AT/Dev/Diamond/BP_Diamond.BP_Diamond_C|SetCan_Be_Grabbed_Flag (Variables|Default|GetContained_Diamond) true)
    (else
      (Variables|/Game/AT/Dev/Diamond/BP_Diamond.BP_Diamond_C|SetCan_Be_Grabbed_Flag (Variables|Default|GetContained_Diamond) false))))

(event Custom|On_Attached_Diamond_Grabbed
  (params (Instigator :type BP%20Diamond%20Object%20Reference))
  (Variables|Default|SetHas_Diamond false))

(event Custom|Set_As_Pivot
  (Default|SetasPivot (Variables|Default|GetContained_Diamond))
  (Default|CallOnSetasPivot))

(event Custom|Set_New_String_Rebuild_State
  (params (New_Moving_State :type EString_Rebuild_State%20Enum :default "NewEnumerator0"))
  (if (Utilities|Enum|NotEqual(Enum) New_Moving_State (Variables|Default|GetString_Rebuild_State))
    (Variables|Default|SetString_Rebuild_State New_Moving_State)
    (switch Utilities|FlowControl|Switch|SwitchonEString_Rebuild_State (Variables|Default|GetString_Rebuild_State)
      (:NewEnumerator4
        (CallFunction|MoveinDirection "NewEnumerator4" (Math|Float|Absolute(Float) (Variables|Default|GetUp_Move_Distance_Local))))
      (:NewEnumerator0
        (CallFunction|MoveinDirection "NewEnumerator0" (Math|Float|Absolute(Float) (Variables|Default|GetBack_Move_Distance_Local))))
      (:NewEnumerator1
        (CallFunction|MoveinDirection "NewEnumerator1" (Variables|Default|GetSide_Move_Distance_Local)))
      (:NewEnumerator2
        (CallFunction|MoveinDirection "NewEnumerator0" (* (Math|Float|Absolute(Float) (Variables|Default|GetBack_Move_Distance_Local)) -1.0)))
      (:NewEnumerator3
        (Variables|Default|SetIs_Moving false)
        (Default|CallOnStopRebuild self)))))

(event Custom|On_Player_In_Interaction_Capsule
  (params (OverlappedComponent :type Primitive%20Component%20Object%20Reference) (OtherActor :type Actor%20Object%20Reference) (OtherComp :type Primitive%20Component%20Object%20Reference) (OtherBodyIndex :type Integer) (bFromSweep :type Boolean) (SweepResult :type Hit%20Result%20Structure%20%28by%20ref%29))
  (Utilities|Casting|CastToBP_Thief OtherActor)
  (Variables|Default|SetIs_Player_In_Capsule true)
  (if (not (Variables|/Game/AT/Dev/Diamond/BP_Diamond.BP_Diamond_C|GetIs_Pivot (Variables|Default|GetContained_Diamond)))
    (Variables|/Game/AT/Dev/Diamond/BP_Diamond.BP_Diamond_C|SetCan_Be_Grabbed_Flag (Variables|Default|GetContained_Diamond) true)))

(event Custom|Move_In_Direction
  (params (Move_Dir :type Move_Direction%20Enum :default "NewEnumerator0") (Distance :type Float%20%28double-precision%29))
  (Variables|Default|SetMove_In_Direction_Distance Distance)
  (Variables|Default|SetIs_Moving true)
  (switch Utilities|FlowControl|Switch|SwitchonMove_Direction Move_Dir
    (:NewEnumerator0
      (Variables|Default|SetMove_Target_Pos (+ (* (Variables|Default|GetMove_In_Direction_Distance) (Transformation|GetActorRightVector)) (Transformation|GetActorLocation))))
    (:NewEnumerator1
      (Variables|Default|SetMove_Target_Pos (+ (* (Variables|Default|GetMove_In_Direction_Distance) (Transformation|GetActorForwardVector)) (Transformation|GetActorLocation))))
    (:NewEnumerator4
      (Variables|Default|SetMove_Target_Pos (+ (* (Variables|Default|GetMove_In_Direction_Distance) (Transformation|GetActorUpVector)) (Transformation|GetActorLocation))))))

(event Custom|On_Player_Leave_Capsule
  (params (OverlappedComponent :type Primitive%20Component%20Object%20Reference) (OtherActor :type Actor%20Object%20Reference) (OtherComp :type Primitive%20Component%20Object%20Reference) (OtherBodyIndex :type Integer))
  (Utilities|Casting|CastToBP_Thief OtherActor)
  (Variables|Default|SetIs_Player_In_Capsule false)
  (Variables|/Game/AT/Dev/Diamond/BP_Diamond.BP_Diamond_C|SetCan_Be_Grabbed_Flag (Variables|Default|GetContained_Diamond) false))

(event EventBeginPlay
  (Collision|BindEventtoOnComponentBeginOverlap (Variables|Default|GetInteraction_Capsule) (delegate Custom|On_Player_In_Interaction_Capsule))
  (Collision|BindEventtoOnComponentEndOverlap (Variables|Default|GetInteraction_Capsule) (delegate Custom|On_Player_Leave_Capsule)))

(event Collision|EventActorBeginOverlap
  (params (OtherActor :type Actor%20Object%20Reference)))

(event EventTick
  (params (DeltaSeconds :type Float%20%28single-precision%29))
  (Utilities|FlowControl|Sequence
    (:then_0
      (if (Variables|Default|GetIs_Moving)
        (if (> (Math|Vector|Distance(Vector) (Transformation|GetActorLocation) (Variables|Default|GetMove_Target_Pos)) (Variables|Default|GetAcceptance_Radius))
          (Transformation|SetActorLocation (Math|Interpolation|VInterpTo (Transformation|GetActorLocation) (Variables|Default|GetMove_Target_Pos) DeltaSeconds 3.0) false false)
          (elif (Utilities|Enum|NotEqual(Enum) (Variables|Default|GetString_Rebuild_State) "NewEnumerator3")
            (CallFunction|SetNewStringRebuildState (Utilities|Enum|ByteToEnumEString_Rebuild_State (+ (Variables|Default|GetString_Rebuild_State) 1)))
            (else
              (Variables|Default|SetIs_Moving false)
              (Default|CallOnStopMoving))))))
    (:then_1
      (if (not (Variables|Default|GetHas_Diamond))
        (for _array_element (Collision|GetOverlappingActors (Variables|Default|GetDead_Zone) "/Game/AT/Dev/Diamond/BP_Diamond.BP_Diamond_C" :!class /Script/Engine.PrimitiveComponent)
          (bind _asbp_diamond (Utilities|Casting|CastToBP_Diamond _array_element))
          (if (not (Variables|/Game/AT/Dev/Diamond/BP_Diamond.BP_Diamond_C|GetIs_Grabbed _asbp_diamond))
            (CallFunction|OnAttachDiamond _asbp_diamond)))))))

(fn ConstructionScript)

(fn AttachDiamond
  (params (Diamond :type BP%20Diamond%20Object%20Reference))
  (Physics|SetSimulatePhysics (Variables|/Game/AT/Dev/Diamond/BP_Diamond.BP_Diamond_C|GetDiamond_Mesh Diamond) false)
  (Transformation|AttachComponentToComponent Diamond (Variables|Default|GetPlatform_Mesh) "Diamond_Socket" "SnapToTarget" "SnapToTarget" "KeepWorld" true)
  (return))

(fn CanbeGrabbed
  (params (Hovered_Component :type Primitive%20Component%20Object%20Reference))
  (return false))

(fn GetGrabComponent
  (return 0))