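; Game mode Blueprint for a Quick Sort level, tracking sort progress and gating the thief player's abilities.
; It plays a helper voice or sound cue through the game instance at BeginPlay and when the first string completes.
; Starting the sort runs once, triggering the first BP_Qick_Sort_Manager found and letting BP_Thief grab diamonds.
; Separate events enable the thief's analyzer and flag sort completion.
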(event Custom|On_String_Complete
  (if (not (Variables|Default|GetIs_First_String_Complete))
    (bind _asat_game_instance (Utilities|Casting|CastToAT_Game_Instance (Game|GetGameInstance)))
    (Default|PlayHelperSoundbyActionSort _asat_game_instance "NewEnumerator12")
    (Variables|Default|SetIs_First_String_Complete true)))

(event Custom|Activate_Analyzer
  (bind _asbp_thief (Utilities|Casting|CastToBP_Thief (Game|Player|GetPlayerPawn 0)))
  (Variables|/Game/AT/Dev/Thief/BP_Thief.BP_Thief_C|SetCan_Use_Analyzer _asbp_thief true))

(event Custom|On_Start_Sorting
  (if (not (Variables|Default|GetIs_Sort_Started))
    (bind _outactors (Actor|GetAllActorsOfClass "/Game/AT/Dev/Quick_Sort/BP_Qick_Sort_Manager.BP_Qick_Sort_Manager_C"))
    (Default|StartSort (Utilities|Array|Get(acopy) _outactors))
    (Variables|Default|SetIs_Sort_Started true)
    (bind _asbp_thief (Utilities|Casting|CastToBP_Thief (Game|Player|GetPlayerPawn 0)))
    (Variables|/Game/AT/Dev/Thief/BP_Thief.BP_Thief_C|SetCan_Grab_Diamonds _asbp_thief true)))

(event Custom|Sort_Complete
  (Variables|Default|SetIs_Sort_End true))

(event EventBeginPlay
  (bind _asat_game_instance (Utilities|Casting|CastToAT_Game_Instance (Game|GetGameInstance)))
  (Default|PlayHelperSoundbyActionSort _asat_game_instance "NewEnumerator8"))

(event EventTick
  (params (DeltaSeconds :type Float%20%28single-precision%29)))

(fn ConstructionScript)