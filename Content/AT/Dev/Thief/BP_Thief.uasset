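; BP_Thief is the first-person player character, with Enhanced Input movement, look sensitivity loaded from a save, and a pause menu.
; Each tick, WorldInteractionComponent traces from the viewpoint to find the hovered actor.
; Clicking presses UI widgets, then scans with the toggleable Analyzer if handed, otherwise interacts or grabs through message calls.
; Grabbed objects follow a PhysicsHandle, bags attach by physics constraint, and AlgoVizorComponent runs a timed greedy highlight scan.
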(event Custom|On_End_Pause
  (bind _returnvalue (SaveGame|DoesSaveGameExist (Variables|Default|GetSlot%20Name)))
  (if _returnvalue
    (bind _returnvalue_2 (SaveGame|LoadGamefromSlot (Variables|Default|GetSlot%20Name)))
    (bind _asmouse_save (Utilities|Casting|CastToMouseSave _returnvalue_2))
    (bind _output_get (Variables|Default|SetSensivity (Variables|/Game/AT/Dev/Save/MouseSave.MouseSave_C|GetSensivityInGame _asmouse_save)))
    (Development|PrintString (Utilities|String|ToString(Float) _output_get))
    (else
      (Variables|Default|SetSensivity 1.0))))

(event Custom|Set_Analyzer_Handed
  (params (Is_Handed :type Boolean))
  ;[1 1 1] Toggle Analyzer Handed
  (bind _output_get (Variables|Default|SetIs_Analyzer_Handed Is_Handed))
  (if _output_get
    (Rendering|SetActorHiddenInGame (Variables|Default|GetAnalyzer) false)
    (else
      (Rendering|SetActorHiddenInGame (Variables|Default|GetAnalyzer) true))))

(event Input|EnhancedActionEvents|EnhancedInputActionIA_Move
  (params (ActionValue :type Vector%202D%20Structure) (ElapsedSeconds :type Float%20%28double-precision%29) (TriggeredSeconds :type Float%20%28double-precision%29) (InputAction :type Input%20Action%20Object%20Reference :default "/Game/AT/Dev/Thief/Input/IA/IA_Move.IA_Move"))
  (bind (_x _y) (Math|Vector2D|BreakVector2D ActionValue))
  ;[1 1 1] Base Movement
  (Pawn|Input|AddMovementInput (+ (* _x (Math|Vector|GetForwardVector (Variables|Default|GetCamera))) (* _y (Math|Vector|GetRightVector (Variables|Default|GetCamera)))) 1.0 false))

(event Input|EnhancedActionEvents|EnhancedInputActionIA_Look
  (params (ActionValue :type Vector%202D%20Structure) (ElapsedSeconds :type Float%20%28double-precision%29) (TriggeredSeconds :type Float%20%28double-precision%29) (InputAction :type Input%20Action%20Object%20Reference :default "/Game/AT/Dev/Thief/Input/IA/IA_Look.IA_Look"))
  (bind (_x _y) (Math|Vector2D|BreakVector2D ActionValue))
  (bind _sensivity (Variables|Default|GetSensivity))
  ;[1 1 1] Base Movement
  (Pawn|Input|AddControllerYawInput (* _x _sensivity))
  (Pawn|Input|AddControllerPitchInput (* _y _sensivity)))

(event Input|EnhancedActionEvents|EnhancedInputActionIA_Mouse_Interact
  (params (ActionValue :type Boolean) (ElapsedSeconds :type Float%20%28double-precision%29) (TriggeredSeconds :type Float%20%28double-precision%29) (InputAction :type Input%20Action%20Object%20Reference :default "/Game/AT/Dev/Thief/Input/IA/IA_Mouse_Interact.IA_Mouse_Interact"))
  (bind _world_interaction_component (Variables|Default|GetWorld_Interaction_Component))
  (bind _hovered_component (Variables|/Game/AT/Dev/Components/BP_World_Interaction_Component.BP_World_Interaction_Component_C|GetHovered_Component _world_interaction_component))
  (bind _hovered_actor (Variables|/Game/AT/Dev/Components/BP_World_Interaction_Component.BP_World_Interaction_Component_C|GetHovered_Actor _world_interaction_component))
  (:Started
    ;[1 1 1] UI
    (Class|WidgetInteractionComponent|PressPointerKey (Variables|Default|GetWidget_Interaction) "LeftMouseButton")
    ;[1 1 1] Analyzer Interaction
    (if (Variables|Default|GetIs_Analyzer_Handed)
      (Default|Scan (Variables|Default|GetAnalyzer) (Variables|/Game/AT/Dev/Components/BP_World_Interaction_Component.BP_World_Interaction_Component_C|GetHovered_Actor (Variables|Default|GetWorld_Interaction_Component)))
      (else
        ;[1 1 1] Grab Actor
        (Utilities|IsValid _hovered_actor
          (:Is%20Valid
            (bind _can_be_grabbed_flag (Class|BPWorldInteractionInterface|CanbeGrabbed(Message) _hovered_actor _hovered_component))
            (if _can_be_grabbed_flag
              (bind _output_get (Variables|Default|SetGrabbed_Actor _hovered_actor))
              (bind _asbp_bag (Utilities|Casting|CastToBP_Bag _output_get)
                (:then
                  (Variables|Default|SetGrabbed_Bag _asbp_bag)
                  (Physics|SetSimulatePhysics (Variables|/Game/AT/Dev/Bag/BP_Bag.BP_Bag_C|GetBag_Mesh (Variables|Default|GetGrabbed_Bag)) true)
                  (Class|PhysicsConstraintComponent|SetConstrainedComponents (Variables|Default|GetBag_Constraint) (Variables|/Game/AT/Dev/Bag/BP_Bag.BP_Bag_C|GetBag_Mesh (Variables|Default|GetGrabbed_Bag)) "None" (Variables|Collision|GetCapsuleComponent) "None")
                  (Variables|Default|SetIs_Grabbed_Bag true)
                  (Variables|Default|SetHas_Grabbed_Actor false))
                (:CastFailed
                  (if (Variables|Default|GetCan_Interact)
                    (Class|BPWorldInteractionInterface|OnGrabbed(Message) _output_get self)
                    (bind _grab_component (Class|BPWorldInteractionInterface|GetGrabComponent(Message) (Variables|Default|GetGrabbed_Actor)))
                    (Physics|Components|PhysicsHandle|GrabComponentatLocationwithRotation (Variables|Default|GetPhysicsHandle) _grab_component "None" (Transformation|GetWorldLocation _grab_component) "0, 0, 0")
                    (Variables|Default|SetHas_Grabbed_Actor true))))
              (else
                (Class|BPWorldInteractionInterface|Interact(Message) _hovered_actor _hovered_component))))))))
  (:Completed
    (Class|WidgetInteractionComponent|ReleasePointerKey (Variables|Default|GetWidget_Interaction) "LeftMouseButton")
    ;[1 1 1] Drop Actor
    (Variables|Default|SetHas_Grabbed_Actor false)
    (Utilities|IsValid (Variables|Default|GetGrabbed_Actor)
      (:Is%20Valid
        (if (Variables|Default|GetIs_Grabbed_Bag)
          (Class|PhysicsConstraintComponent|BreakConstraint (Variables|Default|GetBag_Constraint))
          (Physics|SetSimulatePhysics (Variables|/Game/AT/Dev/Bag/BP_Bag.BP_Bag_C|GetBag_Mesh (Variables|Default|GetGrabbed_Bag)) false)
          (Variables|Default|SetIs_Grabbed_Bag false)
          (else
            (Physics|Components|PhysicsHandle|ReleaseComponent (Variables|Default|GetPhysicsHandle))))
        (Class|BPWorldInteractionInterface|OnDropped(Message) (Variables|Default|GetGrabbed_Actor))
        (Variables|Default|SetGrabbed_Actor 0)))))

(event Input|EnhancedActionEvents|EnhancedInputActionIA_Algo_Vizor
  (params (ActionValue :type Boolean) (ElapsedSeconds :type Float%20%28double-precision%29) (TriggeredSeconds :type Float%20%28double-precision%29) (InputAction :type Input%20Action%20Object%20Reference :default "/Game/AT/Dev/Thief/Input/IA/IA_Algo_Vizor.IA_Algo_Vizor"))
  ;[1 1 1] Algo Vizor
  (:Started
    (Default|GreedyScan (Variables|Default|GetAlgo_Vizor_Component) (Variables|Default|GetVizor_Highlight_Time))))

(event Input|EnhancedActionEvents|EnhancedInputActionIA_Pause
  (params (ActionValue :type Vector%202D%20Structure) (ElapsedSeconds :type Float%20%28double-precision%29) (TriggeredSeconds :type Float%20%28double-precision%29) (InputAction :type Input%20Action%20Object%20Reference :default "/Game/AT/Dev/Thief/Input/IA/IA_Pause.IA_Pause"))
  (bind _returnvalue (UserInterface|CreateWidget "/Game/UI/PauseMenu.PauseMenu_C"))
  (bind _output_get (Variables|Default|SetPauseWidget _returnvalue))
  (UserInterface|Viewport|AddtoViewport _output_get 0)
  (Variables|/Script/Engine.PlayerController|SetbShowMouseCursor (Game|GetPlayerController 0) true)
  (EventDispatchers|BindEventtoOnPauseEnd (Variables|Default|GetPauseWidget) (delegate Custom|On_End_Pause))
  (bind _asat_game_instance (Utilities|Casting|CastToAT_Game_Instance (Game|GetGameInstance)))
  (bind _returnvalue_2 (Game|SetGamePaused true))
  (Class|AudioComponent|SetPaused (Variables|/Game/AT/Dev/Game_Instance/AT_Game_Instance.AT_Game_Instance_C|GetAudio _asat_game_instance) _returnvalue_2))

(event Input|EnhancedActionEvents|EnhancedInputActionIA_Toggle_Analyzer
  (params (ActionValue :type Boolean) (ElapsedSeconds :type Float%20%28double-precision%29) (TriggeredSeconds :type Float%20%28double-precision%29) (InputAction :type Input%20Action%20Object%20Reference :default "/Game/AT/Dev/Thief/Input/IA/IA_Toggle_Analyzer.IA_Toggle_Analyzer"))
  ;[1 1 1] Toggle Analyzer Handed
  (:Started
    (if (Variables|Default|GetCan_Use_Analyzer)
      (Utilities|Casting|CastToGM_Qick_Sort (Game|GetGameMode))
      (if (Variables|Default|GetIs_Analyzer_First_In_Hands)
        (bind _asat_game_instance (Utilities|Casting|CastToAT_Game_Instance (Game|GetGameInstance)))
        (Default|PlayHelperSoundbyActionSort _asat_game_instance "NewEnumerator18")
        (Variables|Default|SetIs_Analyzer_First_In_Hands false))
      (CallFunction|SetAnalyzerHanded (not (Variables|Default|GetIs_Analyzer_Handed))))))

(event EventBeginPlay
  (Input|AddMappingContext (PlayerController|LocalPlayerSubsystems|GetEnhancedInputLocalPlayerSubsystem (Game|GetPlayerController 0)) "/Game/AT/Dev/Thief/Input/IMC_Thief.IMC_Thief" 0 "(bIgnoreAllPressedKeysUntilRelease=True,bForceImmediately=False,bNotifyUserSettings=False)")
  (bind _returnvalue (Game|SpawnActorfromClass "/Game/Props/BP_Analyzer.BP_Analyzer_C" (Math|Transform|MakeTransform "0, 0, 0") "Undefined" "MultiplyWithRoot" 0 0))
  (Variables|Default|SetAnalyzer _returnvalue)
  (Transformation|AttachComponentToComponent (Variables|Default|GetAnalyzer) (Variables|Default|GetAnalyzer_Scene) "None" "SnapToTarget" "SnapToTarget" "SnapToTarget" true)
  (CallFunction|SetAnalyzerHanded false)
  (bind _returnvalue_2 (SaveGame|DoesSaveGameExist (Variables|Default|GetSlot%20Name)))
  (if _returnvalue_2
    (bind _returnvalue_3 (SaveGame|LoadGamefromSlot (Variables|Default|GetSlot%20Name)))
    (bind _asmouse_save (Utilities|Casting|CastToMouseSave _returnvalue_3))
    (Variables|Default|SetSensivity (Variables|/Game/AT/Dev/Save/MouseSave.MouseSave_C|GetSensivityInGame _asmouse_save))
    (else
      (Variables|Default|SetSensivity 1.0))))

(event EventTick
  (params (DeltaSeconds :type Float%20%28single-precision%29))
  (bind _returnvalue (Game|GetPlayerController 0))
  (bind (_location _rotation) (Pawn|GetPlayerViewPoint _returnvalue))
  ;[1 1 1] World Interaction Line Trace
  (Default|Trace (Variables|Default|GetWorld_Interaction_Component) _location (Math|Vector|GetForwardVector _rotation) (Variables|Default|GetInteraction_Trace_Length) (Utilities|Array|MakeArray (Variables|Default|GetAnalyzer) self))
  (if (Variables|Default|GetHas_Grabbed_Actor)
    ;[1 1 1] Update Grabbed Actor Target Pos
    (Class|PhysicsHandleComponent|SetTargetLocationandRotation (Variables|Default|GetPhysicsHandle) (Transformation|GetWorldLocation (Variables|Default|GetGrabbed_Actor_Target)) "0, 0, 0")
    ;[1 1 1] Update Grabbed Actor Rotation
    (Transformation|SetActorRotation (Variables|Default|GetGrabbed_Actor) (Math|Interpolation|RInterpTo (Transformation|GetActorRotation (Variables|Default|GetGrabbed_Actor)) "0, 0, 0" (Utilities|Time|GetWorldDeltaSeconds) (Variables|Default|GetGrabbed_Actor_Rotation_Speed)) true)))

(fn ConstructionScript)