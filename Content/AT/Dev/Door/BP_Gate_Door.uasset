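; BP_Gate_Door is a double gate that also serves as a level exit for the thief.
; Open hides the bar plank, disables its collision and sets a target rotation, which Tick eases both leaves toward in mirrored directions with RInterpTo.
; When BP_Thief overlaps NextLevel, the GM_Qick_Sort game mode loads Lev_Treasure_2_0, while GM_Treasury shows the result.
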(event Custom|Open
  (Development|SetHiddeninGame (Variables|Default|GetMOD_Gateway_Door_01_large_plank_03) true true)
  (Collision|SetCollisionEnabled (Variables|Default|GetMOD_Gateway_Door_01_large_plank_03) "NoCollision")
  (Variables|Default|SetTarget_Rotation "0.000000,90.000000,0.000000"))

(event Custom|On_Next_Level
  (params (OverlappedComponent :type Primitive%20Component%20Object%20Reference) (OtherActor :type Actor%20Object%20Reference) (OtherComp :type Primitive%20Component%20Object%20Reference) (OtherBodyIndex :type Integer) (bFromSweep :type Boolean) (SweepResult :type Hit%20Result%20Structure%20%28by%20ref%29))
  (Utilities|Casting|CastToBP_Thief OtherActor)
  (Utilities|FlowControl|Sequence
    (:then_0
      (Utilities|Casting|CastToGM_Qick_Sort (Game|GetGameMode))
      (Game|OpenLevel(byName) "Lev_Treasure_2_0"))
    (:then_1
      (bind _asgm_treasury (Utilities|Casting|CastToGM_Treasury (Game|GetGameMode)))
      (Default|OnShowResult _asgm_treasury))))

(event EventBeginPlay
  (Collision|BindEventtoOnComponentBeginOverlap (Variables|Default|GetNext_Level) (delegate Custom|On_Next_Level)))

(event Collision|EventActorBeginOverlap
  (params (OtherActor :type Actor%20Object%20Reference)))

(event EventTick
  (params (DeltaSeconds :type Float%20%28single-precision%29))
  (Transformation|SetRelativeRotation (Variables|Default|GetMOD_Gateway_Door_01_large_door_R) (Math|Interpolation|RInterpTo (Variables|/Script/Engine.SceneComponent|GetRelativeRotation (Variables|Default|GetMOD_Gateway_Door_01_large_door_R)) (* (Variables|Default|GetTarget_Rotation) -1.0) (Utilities|Time|GetWorldDeltaSeconds) (Variables|Default|GetInterp_Speed)) false false)
  (Transformation|SetRelativeRotation (Variables|Default|GetMOD_Gateway_Door_01_large_door_L) (Math|Interpolation|RInterpTo (Variables|/Script/Engine.SceneComponent|GetRelativeRotation (Variables|Default|GetMOD_Gateway_Door_01_large_door_L)) (Variables|Default|GetTarget_Rotation) (Utilities|Time|GetWorldDeltaSeconds) 1.0) false false))

(fn ConstructionScript)