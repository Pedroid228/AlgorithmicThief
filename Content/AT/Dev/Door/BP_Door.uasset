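; Interactable, non-grabbable exit door that ends a level when its Stick component is used with the BP_Bag close by.
; Caches the first BP_Bag at BeginPlay and compares its distance to MinBagDistance on interaction.
; With the bag in range, a lab door opens MainMenuMap and other doors show the GM_Treasury result.
; Otherwise it plays a helper sound through the game instance, on lab doors only once GM_Qick_Sort reports sorting finished.
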(event EventBeginPlay
  (bind _outactors (Actor|GetAllActorsOfClass "/Game/AT/Dev/Bag/BP_Bag.BP_Bag_C"))
  (Variables|Default|SetBag (Utilities|Array|Get(acopy) _outactors)))

(event Collision|EventActorBeginOverlap
  (params (OtherActor :type Actor%20Object%20Reference)))

(event EventTick
  (params (DeltaSeconds :type Float%20%28single-precision%29)))

(event EventInteract
  (params (Interaction_Component :type Actor%20Component%20Object%20Reference))
  (if (== Interaction_Component (Variables|Default|GetStick))
    (if (<= (Math|Vector|Distance(Vector) (Transformation|GetActorLocation (Variables|Default|GetBag)) (Transformation|GetActorLocation)) (Variables|Default|GetMin_Bag_Distance))
      (if (Variables|Default|GetIs_Lab_Door)
        (Game|OpenLevel(byName) "MainMenuMap")
        (else
          ;[0.15 0.15 0.15 0.5] Treasure end
          (bind _asgm_treasury (Utilities|Casting|CastToGM_Treasury (Game|GetGameMode)))
          (Default|OnShowResult _asgm_treasury)))
      (else
        ;[0.15 0.15 0.15 0.5] Bag so far
        (if (Variables|Default|GetIs_Lab_Door)
          (bind _asgm_qick_sort (Utilities|Casting|CastToGM_Qick_Sort (Game|GetGameMode)))
          (if (Variables|/Game/AT/Dev/Quick_Sort/GM_Qick_Sort.GM_Qick_Sort_C|GetIs_Sort_End _asgm_qick_sort)
            (bind _asat_game_instance (Utilities|Casting|CastToAT_Game_Instance (Game|GetGameInstance) :!label _label))
            (Default|PlayHelperSoundbyActionTreasury _asat_game_instance "NewEnumerator9"))
          (else
            (goto _label)))))))

(fn ConstructionScript)

(fn CanbeGrabbed
  (params (Hovered_Component :type Primitive%20Component%20Object%20Reference))
  (return false))

(fn GetGrabComponent
  (return 0))