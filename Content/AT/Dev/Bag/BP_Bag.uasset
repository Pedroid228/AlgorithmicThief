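; Grabbable diamond bag that swallows BP_Diamond actors overlapping its DeadZone, hiding them and disabling their physics.
; Regular bags enforce a weight limit and lab bags a CanAddDiamondInLab flag; rejected diamonds are launched from PopStart with a random impulse.
; Pop_Diamond ejects the last stored diamond likewise, though its pop-panel binding is disconnected.
; Dispatchers broadcast content and fill changes, while the game instance plays helper voice cues.
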(event Custom|Try_Add_Diamond
  (params (OverlappedComponent :type Primitive%20Component%20Object%20Reference) (OtherActor :type Actor%20Object%20Reference) (OtherComp :type Primitive%20Component%20Object%20Reference) (OtherBodyIndex :type Integer) (bFromSweep :type Boolean) (SweepResult :type Hit%20Result%20Structure%20%28by%20ref%29))
  ;[1 1 1] Push
  (bind _asbp_diamond (Utilities|Casting|CastToBP_Diamond OtherActor))
  (Variables|Default|SetNew_Diamond _asbp_diamond)
  (if (Variables|Default|GetIs_Lab_Bag)
    (if (Variables|Default|GetCan_Add_Diamond_In_Lab)
      (Rendering|SetActorHiddenInGame (Variables|Default|GetNew_Diamond) true :!label _label)
      (Collision|SetCollisionEnabled (Variables|/Game/AT/Dev/Diamond/BP_Diamond.BP_Diamond_C|GetDiamond_Mesh (Variables|Default|GetNew_Diamond)) "NoCollision")
      (Physics|SetSimulatePhysics (Variables|/Game/AT/Dev/Diamond/BP_Diamond.BP_Diamond_C|GetDiamond_Mesh (Variables|Default|GetNew_Diamond)) false)
      (Variables|/Game/AT/Dev/Diamond/BP_Diamond.BP_Diamond_C|SetIs_In_Bag (Variables|Default|GetNew_Diamond) true)
      (Utilities|Array|Add (Variables|Default|GetDiamonds) (Variables|Default|GetNew_Diamond))
      (CallFunction|OnWeightChanged)
      (Default|CallOnContainedDiamondsUpdated (Variables|Default|GetDiamonds))
      (Audio|PlaySound2D "/Game/Audio/Sfx/diamond_in_bag_sound.diamond_in_bag_sound" 1.0 1.0 0.0 0 0)
      (if (Variables|Default|GetIs_First_Diamond_In_Bag)
        (Variables|Default|SetIs_First_Diamond_In_Bag false)
        (bind _asat_game_instance (Utilities|Casting|CastToAT_Game_Instance (Game|GetGameInstance)))
        (Default|PlayHelperSoundbyActionTreasury _asat_game_instance "NewEnumerator11"))
      (else
        ;[1 1 1] No space in bag
        (Physics|SetSimulatePhysics (Variables|/Game/AT/Dev/Diamond/BP_Diamond.BP_Diamond_C|GetDiamond_Mesh (Variables|Default|GetNew_Diamond)) false :!label _label_2)
        (Transformation|SetActorLocationAndRotation (Variables|Default|GetNew_Diamond) (Transformation|GetWorldLocation (Variables|Default|GetPop_Start)))
        (Physics|SetSimulatePhysics (Variables|/Game/AT/Dev/Diamond/BP_Diamond.BP_Diamond_C|GetDiamond_Mesh (Variables|Default|GetNew_Diamond)) true)
        (Physics|AddImpulse (Variables|/Game/AT/Dev/Diamond/BP_Diamond.BP_Diamond_C|GetDiamond_Mesh (Variables|Default|GetNew_Diamond)) (Math|Vector|MakeVector (Math|Random|RandomFloatinRange 5e+02 1.5e+03) (Math|Random|RandomFloatinRange 0.0 1.5e+03) 6e+03) "None" false)
        (if (Variables|Default|GetIs_Lab_Bag)
          (bind _asat_game_instance_2 (Utilities|Casting|CastToAT_Game_Instance (Game|GetGameInstance)))
          (Default|PlayHelperSoundbyActionSort _asat_game_instance_2 "NewEnumerator19")
          (elif (Variables|Default|GetIs_First_Bag_Full)
            (bind _asat_game_instance_3 (Utilities|Casting|CastToAT_Game_Instance (Game|GetGameInstance)))
            (Default|PlayHelperSoundbyActionTreasury _asat_game_instance_3 "NewEnumerator0")
            (Variables|Default|SetIs_First_Bag_Full false)))))
    (elif (<= (+ (Variables|Default|GetCurr_Weight) (.Weight (Utilities|Struct|BreakSDiamond_Data (Variables|/Game/AT/Dev/Diamond/BP_Diamond.BP_Diamond_C|GetDiamond_Data (Variables|Default|GetNew_Diamond))))) (Variables|Default|GetMax_Weight))
      (Variables|Default|SetCurr_Weight (+ (Variables|Default|GetCurr_Weight) (.Weight (Utilities|Struct|BreakSDiamond_Data (Variables|/Game/AT/Dev/Diamond/BP_Diamond.BP_Diamond_C|GetDiamond_Data (Variables|Default|GetNew_Diamond))))))
      (goto _label)
      (else
        (goto _label_2)))))

(event Custom|Pop_Diamond
  (bind _diamonds (Variables|Default|GetDiamonds))
  (bind _diamonds_2 (Variables|Default|GetDiamonds))
  (bind _returnvalue (Utilities|Array|LastIndex _diamonds_2))
  (bind _output (Utilities|Array|Get(acopy) _diamonds _returnvalue))
  ;[1 1 1] Pop
  (Utilities|IsValid _output
    (:Is%20Valid
      (bind _output_get (Variables|Default|SetCurr_Pop_Diamond _output))
      (Transformation|SetActorLocationAndRotation _output_get (Transformation|GetWorldLocation (Variables|Default|GetPop_Start)))
      (Rendering|SetActorHiddenInGame (Variables|Default|GetCurr_Pop_Diamond) false)
      (Collision|SetCollisionEnabled (Variables|/Game/AT/Dev/Diamond/BP_Diamond.BP_Diamond_C|GetDiamond_Mesh (Variables|Default|GetCurr_Pop_Diamond)) "QueryAndPhysics")
      (Physics|SetSimulatePhysics (Variables|/Game/AT/Dev/Diamond/BP_Diamond.BP_Diamond_C|GetDiamond_Mesh (Variables|Default|GetCurr_Pop_Diamond)) true)
      (Physics|AddImpulse (Variables|/Game/AT/Dev/Diamond/BP_Diamond.BP_Diamond_C|GetDiamond_Mesh (Variables|Default|GetCurr_Pop_Diamond)) (Math|Vector|MakeVector (Math|Random|RandomFloatinRange 5e+02 1.5e+03) (Math|Random|RandomFloatinRange 0.0 1.5e+03) 6e+03) "None" false)
      (Variables|/Game/AT/Dev/Diamond/BP_Diamond.BP_Diamond_C|SetIs_In_Bag (Variables|Default|GetCurr_Pop_Diamond) false)
      (Variables|Default|SetCurr_Weight (- (Variables|Default|GetCurr_Weight) (.Weight (Utilities|Struct|BreakSDiamond_Data (Variables|/Game/AT/Dev/Diamond/BP_Diamond.BP_Diamond_C|GetDiamond_Data (Variables|Default|GetCurr_Pop_Diamond))))))
      (Utilities|Array|RemoveIndex (Variables|Default|GetDiamonds) (Utilities|Array|LastIndex (Variables|Default|GetDiamonds)))
      (CallFunction|OnWeightChanged)
      (Default|CallOnContainedDiamondsUpdated (Variables|Default|GetDiamonds)))))

(event EventBeginPlay
  (Collision|AssignOnComponentBeginOverlap (Variables|Default|GetDead_Zone) (delegate Custom|Try_Add_Diamond)))

(fn ConstructionScript)

(fn OnWeightChanged
  (Default|CallOnWeightChangedDispatch (Math|Float|Clamp(Float) (/ (Variables|Default|GetCurr_Weight) (Variables|Default|GetMax_Weight))) (Variables|Default|GetCurr_Weight)))

(fn CanbeGrabbed
  (params (Hovered_Component :type Primitive%20Component%20Object%20Reference))
  (return (== Hovered_Component (Variables|Default|GetBag_Mesh))))

(fn GetGrabComponent
  (return (Variables|Default|GetBag_Mesh)))