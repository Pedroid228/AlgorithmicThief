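; Player controller for the Treasury that detects when the player's pawn stands idle and plays a helper sound.
; Each tick it compares the pawn's location with the last stored one, accumulating idle time while unchanged and resetting it on movement.
; When idle time reaches the detection threshold, it asks the AT game instance to play a Treasury action helper sound, then restarts the timer.
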(event EventBeginPlay)

(event EventTick
  (params (DeltaSeconds :type Float%20%28single-precision%29))
  (if (Utilities|Operators|EqualEqual (Variables|Default|GetLast_Location) (Transformation|GetActorLocation (Game|Player|GetPlayerPawn 0)) 0.001)
    (bind _output_get (Variables|Default|SetCurr_Idle_Time (+ (Variables|Default|GetCurr_Idle_Time) (Utilities|Time|GetWorldDeltaSeconds))))
    (if (>= _output_get (Variables|Default|GetIdle_Detect_Time))
      (bind _asat_game_instance (Utilities|Casting|CastToAT_Game_Instance (Game|GetGameInstance)))
      (Default|PlayHelperSoundbyActionTreasury _asat_game_instance "NewEnumerator1")
      (Variables|Default|SetCurr_Idle_Time 0.0))
    (else
      (Variables|Default|SetCurr_Idle_Time 0.0)))
  (Variables|Default|SetLast_Location (Transformation|GetActorLocation (Game|Player|GetPlayerPawn 0))))

(fn ConstructionScript)