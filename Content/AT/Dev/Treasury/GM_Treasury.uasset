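; Game mode for the Treasury level, a timed diamond heist that plays like a knapsack puzzle.
; Start_Robbery enables grabbing and starts a Tick countdown with helper voice cues; expiry disables grabbing and opens the gate.
; Bag dispatchers update the HUD, and the result screen receives the player's haul plus optimal and greedy sets spawned from stored data.
; An in-graph greedy price-per-weight bubble sort and bag fill is left disconnected.
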(event Custom|Start_Robbery
  (params (Instigator :type BP%20Diamond%20Object%20Reference))
  (if (not (Variables|Default|GetIs_Robbery_Started))
    (Variables|Default|SetIs_Robbery_Started true)
    (Audio|PlaySound2D "/Game/Audio/Music/treasury_sound.treasury_sound" 0.5 1.0 0.0 0 0 false)
    (Utilities|FlowControl|Sequence
      (:then_0
        ;[1 1 1] Unbind event
        (for _array_element (Variables|Default|GetDiamonds)
          (EventDispatchers|UnbindEventfromOnGrabbedDispatcher _array_element (delegate Custom|Start_Robbery))))
      (:then_1
        (Variables|Default|SetCurr_Time (Variables|Default|GetRobbery_Time))
        (Variables|Default|SetIs_Robbery_In_Progress true))
      (:then_2
        (bind _asbp_thief (Utilities|Casting|CastToBP_Thief (Pawn|GetControlledPawn (Game|GetPlayerController 0))))
        (Variables|/Game/AT/Dev/Thief/BP_Thief.BP_Thief_C|SetCan_Grab_Diamonds _asbp_thief true)))))

(event Custom|On_Bag_Filling_Ratio_Update
  (params (New_Filling_Ratio :type Float%20%28double-precision%29) (New_Weight :type Float%20%28double-precision%29))
  (Default|UpdateBagFillingRatio (Variables|Default|GetTreasury_HUD) New_Filling_Ratio New_Weight))

(event Custom|On_Bag_Contains_Updated
  (params (Contained_Diamonds :type Array%20of%20BP%20Diamond%20Object%20References))
  (Default|UpdateBagStack (Variables|Default|GetTreasury_HUD) Contained_Diamonds))

(event Custom|On_End_Robbery
  (bind _asbp_thief (Utilities|Casting|CastToBP_Thief (Pawn|GetControlledPawn (Game|GetPlayerController 0))))
  (Variables|/Game/AT/Dev/Thief/BP_Thief.BP_Thief_C|SetCan_Grab_Diamonds _asbp_thief false)
  (bind _asat_game_instance (Utilities|Casting|CastToAT_Game_Instance (Game|GetGameInstance)))
  (Default|PlayHelperSoundbyActionTreasury _asat_game_instance "NewEnumerator8")
  (bind _outactors (Actor|GetAllActorsOfClass "/Game/AT/Dev/Door/BP_Gate_Door.BP_Gate_Door_C"))
  (Default|Open (Utilities|Array|Get(acopy) _outactors)))

(event Custom|On_Show_Result
  (bind _bag (Variables|Default|GetBag))
  (Utilities|FlowControl|Sequence
    (:then_0
      (for _array_element (Variables|Default|GetOptimal_Diamonds_Data)
        (bind _returnvalue (Game|SpawnActorfromClass "/Game/AT/Dev/Diamond/BP_Diamond.BP_Diamond_C" (Math|Transform|MakeTransform "0, 0, 0") "Undefined" "MultiplyWithRoot" 0 0))
        (Variables|/Game/AT/Dev/Diamond/BP_Diamond.BP_Diamond_C|SetDiamond_Data _returnvalue _array_element)
        (Utilities|Array|Add (Variables|Default|GetOptimal_Diamonds) _returnvalue)))
    (:then_1
      (for _array_element_2 (Variables|Default|GetGreed_Diamonds_Data)
        (bind _returnvalue_2 (Game|SpawnActorfromClass "/Game/AT/Dev/Diamond/BP_Diamond.BP_Diamond_C" (Math|Transform|MakeTransform "0, 0, 0") "Undefined" "MultiplyWithRoot" 0 0))
        (Variables|/Game/AT/Dev/Diamond/BP_Diamond.BP_Diamond_C|SetDiamond_Data _returnvalue_2 _array_element_2)
        (Utilities|Array|Add (Variables|Default|GetGreed_Diamonds) _returnvalue_2)))
    (:then_2
      (Default|ShowTreasureEnd (Variables|Default|GetTreasury_HUD) (Variables|/Game/AT/Dev/Bag/BP_Bag.BP_Bag_C|GetDiamonds _bag) (Variables|Default|GetOptimal_Diamonds) (Variables|Default|GetGreed_Diamonds) (Variables|/Game/AT/Dev/Bag/BP_Bag.BP_Bag_C|GetMax_Weight _bag)))))

(event EventBeginPlay
  (Utilities|FlowControl|Sequence
    (:then_0
      (bind _asbp_thief (Utilities|Casting|CastToBP_Thief (Pawn|GetControlledPawn (Game|GetPlayerController 0))))
      (Variables|/Game/AT/Dev/Thief/BP_Thief.BP_Thief_C|SetCan_Grab_Diamonds _asbp_thief false)
      (Variables|/Game/AT/Dev/Thief/BP_Thief.BP_Thief_C|SetCan_Drop_Diamond _asbp_thief true))
    (:then_1
      (bind _asat_game_instance (Utilities|Casting|CastToAT_Game_Instance (Game|GetGameInstance)))
      (Default|PlayHelperSoundbyActionTreasury _asat_game_instance "NewEnumerator2")
      (bind _outactors (Actor|GetAllActorsOfClass "/Game/AT/Dev/Diamond/BP_Diamond.BP_Diamond_C"))
      (Variables|Default|SetDiamonds _outactors)
      (bind _astreasury_hud (Utilities|Casting|CastToTreasury_HUD (HUD|GetHUD (Game|GetPlayerController 0))))
      (bind _output_get (Variables|Default|SetTreasury_HUD _astreasury_hud))
      (Default|Setup _output_get (Variables|Default|GetRobbery_Time)))
    (:then_2
      ;[1 1 1] Bag
      (bind _outactors_2 (Actor|GetAllActorsOfClass "/Game/AT/Dev/Bag/BP_Bag.BP_Bag_C"))
      (bind _output_get_2 (Variables|Default|SetBag (Utilities|Array|Get(acopy) _outactors_2)))
      (EventDispatchers|BindEventtoOnWeightChangedDispatch _output_get_2 (delegate Custom|On_Bag_Filling_Ratio_Update))
      (EventDispatchers|BindEventtoOnContainedDiamondsUpdated (Variables|Default|GetBag) (delegate Custom|On_Bag_Contains_Updated)))))

(event EventTick
  (params (DeltaSeconds :type Float%20%28single-precision%29))
  (Variables|Default|SetDelta_Seconds_Local DeltaSeconds)
  (if (Variables|Default|GetIs_Robbery_In_Progress)
    (Variables|Default|SetCurr_Time (- (Variables|Default|GetCurr_Time) (Variables|Default|GetDelta_Seconds_Local)))
    (Utilities|FlowControl|Sequence
      (:then_0
        (if (<= (Variables|Default|GetCurr_Time) (/ (Variables|Default|GetRobbery_Time) 2.0))
          (if (Variables|Default|GetIs_First_Half_Time)
            (Variables|Default|SetIs_First_Half_Time false)
            (bind _asat_game_instance (Utilities|Casting|CastToAT_Game_Instance (Game|GetGameInstance)))
            (Default|PlayHelperSoundbyActionTreasury _asat_game_instance "NewEnumerator12"))))
      (:then_1
        (if (<= (Variables|Default|GetCurr_Time) 1e+01)
          (if (Variables|Default|GetIs_First_Ten_Seconds)
            (Variables|Default|SetIs_First_Ten_Seconds false)
            (bind _asat_game_instance_2 (Utilities|Casting|CastToAT_Game_Instance (Game|GetGameInstance)))
            (Default|PlayHelperSoundbyActionTreasury _asat_game_instance_2 "NewEnumerator13"))))
      (:then_2
        (if (<= (Variables|Default|GetCurr_Time) 0.0)
          (Variables|Default|SetIs_Robbery_In_Progress false)
          (CallFunction|OnEndRobbery)
          (else
            (Default|SetTimerValue (Variables|Default|GetTreasury_HUD) (Variables|Default|GetCurr_Time))))))))

(fn ConstructionScript)