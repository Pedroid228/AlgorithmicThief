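; BP_ThiefBag is a bag prop that marks where the thief can drop a diamond.
; On BeginPlay it makes DiamondHole visible and caches the BP_Thief found in the level.
; When a BP_Diamond begins or ends overlap with the Diamond_Hole component, it sets or clears CanDropDiamond on that thief.
; The bag only toggles this flag and contains no drop logic itself.
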(event OnComponentBeginOverlap(Diamond_Hole)
  (params (OverlappedComponent :type Primitive%20Component%20Object%20Reference) (OtherActor :type Actor%20Object%20Reference) (OtherComp :type Primitive%20Component%20Object%20Reference) (OtherBodyIndex :type Integer) (bFromSweep :type Boolean) (SweepResult :type Hit%20Result%20Structure%20%28by%20ref%29))
  (bind _player (Variables|Default|GetPlayer))
  (Utilities|Casting|CastToBP_Diamond OtherActor)
  (Utilities|IsValid _player
    (:Is%20Valid
      (Variables|/Game/AT/Dev/Thief/BP_Thief.BP_Thief_C|SetCan_Drop_Diamond _player true))))

(event OnComponentEndOverlap(Diamond_Hole)
  (params (OverlappedComponent :type Primitive%20Component%20Object%20Reference) (OtherActor :type Actor%20Object%20Reference) (OtherComp :type Primitive%20Component%20Object%20Reference) (OtherBodyIndex :type Integer))
  (bind _player (Variables|Default|GetPlayer))
  (Utilities|Casting|CastToBP_Diamond OtherActor)
  (Utilities|IsValid _player
    (:Is%20Valid
      (Variables|/Game/AT/Dev/Thief/BP_Thief.BP_Thief_C|SetCan_Drop_Diamond _player false))))

(event EventBeginPlay
  (Development|SetHiddeninGame (Variables|Default|GetDiamond_Hole) false false)
  (bind _returnvalue (Actor|GetActorOfClass "/Game/AT/Dev/Thief/BP_Thief.BP_Thief_C"))
  (Variables|Default|SetPlayer _returnvalue))

(fn ConstructionScript)