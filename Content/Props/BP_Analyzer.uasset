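; BP_Analyzer is a prop that scans a diamond over a timed interval and displays its price on an attached screen widget.
; Scan accepts only a BP_Diamond, caches the screen widget and starts a timer that Tick uses to fill the progress bar.
; On completion it clears the bar, shows the diamond's price, plays a sound and, on the first scan only, triggers a helper voice cue through the game instance.
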(event Custom|Scan
  (params (Scanning_Actor :type Actor%20Object%20Reference))
  (Utilities|IsValid Scanning_Actor
    (:Is%20Valid
      (bind _asbp_diamond (Utilities|Casting|CastToBP_Diamond Scanning_Actor)
        (:then
          (Variables|Default|SetScanning_Diamond _asbp_diamond)
          (Variables|Default|SetIs_Scanning true)
          (Variables|Default|SetCurr_Time 0.0)
          (bind _aswbp_analyzer_screen (Utilities|Casting|CastToWBP_Analyzer_Screen (UserInterface|GetWidget (Variables|Default|GetScreen_Widget))))
          (Variables|Default|SetAnalyzer_Screen_Widget _aswbp_analyzer_screen))
        (:CastFailed
          (Development|PrintString "No Diamond" :!label _label))))
    (:Is%20Not%20Valid
      (goto _label))))

(event EventBeginPlay)

(event Collision|EventActorBeginOverlap
  (params (OtherActor :type Actor%20Object%20Reference)))

(event EventTick
  (params (DeltaSeconds :type Float%20%28single-precision%29))
  (if (Variables|Default|GetIs_Scanning)
    (Variables|Default|SetCurr_Time (+ (Variables|Default|GetCurr_Time) DeltaSeconds))
    (Variables|Default|SetComplete_Ratio (/ (Variables|Default|GetCurr_Time) (Variables|Default|GetScanning_Time)))
    (if (>= (Variables|Default|GetComplete_Ratio) 1.0)
      (Variables|Default|SetIs_Scanning false)
      (Variables|Default|SetComplete_Ratio 0.0)
      (Progress|SetPercent (Variables|/Game/Props/3_Analyzer/Analyzer_Screen/WBP_Analyzer_Screen.WBP_Analyzer_Screen_C|GetScanning_Bar (Variables|Default|GetAnalyzer_Screen_Widget)) (Variables|Default|GetComplete_Ratio))
      (Variables|/Script/UMG.TextBlock|SetText (Variables|/Game/Props/3_Analyzer/Analyzer_Screen/WBP_Analyzer_Screen.WBP_Analyzer_Screen_C|GetPrice_Text (Variables|Default|GetAnalyzer_Screen_Widget)) (Utilities|Text|ToText(Float) (.price (Variables|/Game/AT/Dev/Diamond/BP_Diamond.BP_Diamond_C|GetDiamond_Data (Variables|Default|GetScanning_Diamond))) "HalfToEven"))
      (Audio|PlaySound2D "/Game/Audio/Sfx/analyze_sound.analyze_sound" 1.0 1.0 0.0 0 0)
      (if (Variables|Default|GetIs_First_Scan)
        (Variables|Default|SetIs_First_Scan false)
        (bind _asat_game_instance (Utilities|Casting|CastToAT_Game_Instance (Game|GetGameInstance)))
        (Default|PlayHelperSoundbyActionSort _asat_game_instance "NewEnumerator16"))
      (else
        (Progress|SetPercent (Variables|/Game/Props/3_Analyzer/Analyzer_Screen/WBP_Analyzer_Screen.WBP_Analyzer_Screen_C|GetScanning_Bar (Variables|Default|GetAnalyzer_Screen_Widget)) (Variables|Default|GetComplete_Ratio))))))

(fn ConstructionScript)